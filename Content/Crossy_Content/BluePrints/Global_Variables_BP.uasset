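; Global variables actor for a Crossy Road-style game that tracks the player chicken's forward progress as a level score.
; Every Tick it finds all Chimken actors and compares each capsule's world X to the stored furthest LevelPosition.
; A new furthest X updates that position, adds one point to LevelScore regardless of distance and sets IsIncreasing, which is never cleared here.
; CoinScore and IsDead appear only in unconnected debug prints.
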(event Collision|EventActorBeginOverlap
  (params (OtherActor :type Actor%20Object%20Reference)))

(event EventTick
  (params (DeltaSeconds :type Float%20%28single-precision%29))
  (CallFunction|SetLevelScore))

(fn ConstructionScript)

(fn SetLevelScore
  (bind _outactors (Actor|GetAllActorsOfClass "/Game/Crossy_Content/BluePrints/chimken.chimken_C"))
  (for _array_element _outactors
    (bind _aschimken (Utilities|Casting|CastTochimken _array_element))
    (if (> (.x (Transformation|GetWorldLocation (Variables|/Script/Engine.Character|GetCapsuleComponent _aschimken))) (Variables|Default|GetLevel_Position))
      (Variables|Default|SetLevel_Position (.x (Transformation|GetWorldLocation (Variables|/Script/Engine.Character|GetCapsuleComponent _aschimken))))
      (Variables|Default|SetLevel_Score (+ (Variables|Default|GetLevel_Score) 1))
      (Variables|Default|SetIs_Increasing true))))
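; Truck hazard that drives along a referenced track spline and kills the chicken on contact.
; On BeginPlay, an active truck runs the CartMover timeline from a start offset at a duration-based rate, mapping its alpha to spline position and rotation.
; Any box overlap, unfiltered, flattens the other actor at the truck's location, sets IsDead on Global_Variables_BP and spawns death particles at every Chimken.
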(event OnComponentBeginOverlap(Box)
  (params (OverlappedComponent :type Primitive%20Component%20Object%20Reference) (OtherActor :type Actor%20Object%20Reference) (OtherComp :type Primitive%20Component%20Object%20Reference) (OtherBodyIndex :type Integer) (bFromSweep :type Boolean) (SweepResult :type Hit%20Result%20Structure%20%28by%20ref%29))
  ;[1 1 1] Detects Collision
  (Transformation|SetActorTransform OtherActor (Math|Transform|MakeTransform (Transformation|GetActorLocation) "0, 0, 0" "1.000000,1.000000,0.200000"))
  (bind _outactors (Actor|GetAllActorsOfClass "/Game/Crossy_Content/BluePrints/Global_Variables_BP.Global_Variables_BP_C"))
  (for _array_element _outactors
    (bind _asglobal_variables_bp (Utilities|Casting|CastToGlobal_Variables_BP _array_element))
    (Variables|/Game/Crossy_Content/BluePrints/Global_Variables_BP.Global_Variables_BP_C|SetIs_Dead _asglobal_variables_bp true)
    (bind _outactors_2 (Actor|GetAllActorsOfClass "/Game/Crossy_Content/BluePrints/chimken.chimken_C"))
    (for _array_element_2 _outactors_2
      (bind _aschimken (Utilities|Casting|CastTochimken _array_element_2))
      (Effects|SpawnEmitteratLocation "/Game/Crossy_Content/Particle_System/Chicken_Death.Chicken_Death" (Transformation|GetWorldLocation (Variables|/Script/Engine.Character|GetCapsuleComponent _aschimken))))))

(event Custom|MoveCart
  (Components|Timeline|SetPlayRate (Variables|Default|GetCartMover) (/ 1.0 (Variables|Default|GetDuration)))
  (Components|Timeline|SetNewTime (Variables|Default|GetCartMover) (Variables|Default|GetCartStartOffset))
  (bind _alpha (Timeline|CartMover Play)
    (:Update
      (Variables|Default|SetAlpha _alpha)
      (Transformation|SetActorLocationAndRotation (Spline|GetLocationatDistanceAlongSpline (Variables|/Game/Crossy_Content/BluePrints/Track.Track_C|GetUsefulSpline (Variables|Default|GetTrackRef)) (Math|Float|Lerp 0.0 (Spline|GetSplineLength (Variables|/Game/Crossy_Content/BluePrints/Track.Track_C|GetUsefulSpline (Variables|Default|GetTrackRef))) (Variables|Default|GetAlpha)) "World") (Spline|GetRotationatDistanceAlongSpline (Variables|/Game/Crossy_Content/BluePrints/Track.Track_C|GetUsefulSpline (Variables|Default|GetTrackRef)) (Math|Float|Lerp 0.0 (Spline|GetSplineLength (Variables|/Game/Crossy_Content/BluePrints/Track.Track_C|GetUsefulSpline (Variables|Default|GetTrackRef))) (Variables|Default|GetAlpha)) "World")))))

(event EventBeginPlay
  (if (Variables|Default|GetActiveCart)
    (CallFunction|MoveCart)))

(fn ConstructionScript)
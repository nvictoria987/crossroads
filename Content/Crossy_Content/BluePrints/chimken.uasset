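; Player chicken character for a Crossy Road-style game, hopping with WASD while grounded, with 200-unit grid rounding on some moves.
; Forward hops can unload old streamed levels and request new ones through Global_Variables_BP, based on score.
; Tick follows with the camera, locks grounded height and counts idle frames toward an eagle death.
; When dead, it either resets to origin with a frozen camera or follows Asset1's mesh with blood effects.
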(event EventTick
  (params (DeltaSeconds :type Float%20%28single-precision%29))
  (bind _capsulecomponent (Variables|Collision|GetCapsuleComponent))
  (bind _returnvalue (Transformation|GetWorldLocation _capsulecomponent))
  ;[0.1156 0.3086 1] Movement
  ;;[0 1 0.2434] Delta Time
  ;[1 0.01578 0] Camera Movement
  ;;[1 1 1] Checks if Chicken is alive
  (bind _outactors (Actor|GetAllActorsOfClass "/Game/Crossy_Content/BluePrints/Global_Variables_BP.Global_Variables_BP_C"))
  (for _array_element _outactors
    (bind _asglobal_variables_bp (Utilities|Casting|CastToGlobal_Variables_BP _array_element))
    (if (Variables|/Game/Crossy_Content/BluePrints/Global_Variables_BP.Global_Variables_BP_C|GetIs_Dead _asglobal_variables_bp)
      ;;[1 1 1] If Dead, move chicken to position (0,0,0) and freeze camera
      (if (Variables|Default|Geteagle_death)
        ;;[1 1 1] Camera for Death By Eagle
        (CallFunction|DeathbyEagle)
        (else
          (Transformation|SetWorldLocation (Variables|Collision|GetCapsuleComponent) "0, 0, 0" false false)
          (Transformation|SetWorldLocation (Variables|Default|GetCamera) (Variables|Default|GetCamera_Location) false false)))
      (else
        (Transformation|SetWorldLocation (Variables|Default|GetCamera) (Math|Vector|MakeVector (+ (.x (Transformation|GetWorldLocation (Variables|Default|GetMain_Player))) -4e+02) 0.0 1e+03) false false)
        ;;[1 1 1] Checks if player is on ground, if so locks z axis to 90 (fixes x and y offsets going off grid)
        (if (AI|Components|NavMovement|IsMovingonGround (Variables|Character|GetCharacterMovement))
          ;;[1 1 1] set player location and save camera location
          (Transformation|SetWorldLocation (Variables|Collision|GetCapsuleComponent) (Math|Vector|MakeVector (.x _returnvalue) (.y _returnvalue) 9e+01) false false)
          (Variables|Default|SetCamera_Location (Transformation|GetWorldLocation (Variables|Default|GetCamera)))
          (bind _output_get (Variables|Default|SetIdle_Counter (+ (Variables|Default|GetIdle_Counter) 1)))
          (if (>= _output_get 300)
            (Variables|Default|Seteagle_death true)
            (bind _outactors_2 (Actor|GetAllActorsOfClass "/Game/Crossy_Content/BluePrints/Global_Variables_BP.Global_Variables_BP_C"))
            (for _array_element_2 _outactors_2
              (Variables|/Game/Crossy_Content/BluePrints/Global_Variables_BP.Global_Variables_BP_C|SetIs_Dead _array_element_2 true))))))))

(event Input|KeyboardEvents|W
  (params (Key :type Key%20Structure))
  ;[0.1156 0.3086 1] Movement
  ;;[1 0.1961 0.5725] Up
  (:Pressed
    (if (AI|Components|NavMovement|IsMovingonGround (Variables|Character|GetCharacterMovement))
      (Character|Jump)
      (bind _xvalue (CallFunction|RoundX))
      (bind _yvalue (CallFunction|RoundY))
      (Transformation|SetActorRelativeLocation (Math|Vector|MakeVector (+ _xvalue (* -1.0 (Variables|Default|Getspeed))) _yvalue (.z (Transformation|GetActorLocation))) true)
      (Transformation|SetWorldRotation (Variables|Default|GetMain_Player) "0,270.000000, 0" false false)
      ;;;[1 0 0.1016] Add Delete Levels
      (bind _outactors (Actor|GetAllActorsOfClass "/Game/Crossy_Content/BluePrints/Global_Variables_BP.Global_Variables_BP_C"))
      (for _array_element _outactors
        (if (>= (Variables|/Game/Crossy_Content/BluePrints/Global_Variables_BP.Global_Variables_BP_C|GetLevel_Score _array_element) 5)
          (if (Variables|/Game/Crossy_Content/BluePrints/Global_Variables_BP.Global_Variables_BP_C|GetIs_Increasing _array_element)
            (for (_array_element_2 _array_index) (Variables|Default|GetStore%20Level%20Names)
              (if (== _array_index (Variables|Default|Getcounta))
                (Game|UnloadStreamLevel(byName) _array_element_2 true)
                (Variables|Default|Setcounta (+ (Variables|Default|Getcounta) 1))
                (Variables|/Game/Crossy_Content/BluePrints/Global_Variables_BP.Global_Variables_BP_C|Setcreate_level _array_element true)
                (Variables|Default|SetIdle_Counter 0)))))))))

(event Input|KeyboardEvents|A
  (params (Key :type Key%20Structure))
  (bind _returnvalue (Transformation|GetActorLocation))
  (:Pressed
    (if (AI|Components|NavMovement|IsMovingonGround (Variables|Character|GetCharacterMovement))
      (Character|Jump)
      (Transformation|SetActorRelativeLocation (Math|Vector|MakeVector (.x _returnvalue) (+ (.y _returnvalue) (* 1.0 (Variables|Default|Getspeed))) (.z _returnvalue)) true)
      (Transformation|SetWorldRotation (Variables|Default|GetMain_Player) "0,180.000000, 0" false false))))

(event Input|KeyboardEvents|W
  (params (Key :type Key%20Structure)))

(event Input|KeyboardEvents|S
  (params (Key :type Key%20Structure))
  ;[0.1156 0.3086 1] Movement
  ;;[1 0.1961 0.5725] Down
  (:Pressed
    (if (AI|Components|NavMovement|IsMovingonGround (Variables|Character|GetCharacterMovement))
      (Character|Jump)
      (bind _xvalue (CallFunction|RoundX))
      (bind _yvalue (CallFunction|RoundY))
      (Transformation|SetActorRelativeLocation (Math|Vector|MakeVector (+ _xvalue (* 1.0 (Variables|Default|Getspeed))) _yvalue (.z (Transformation|GetActorLocation))) true)
      (Transformation|SetWorldRotation (Variables|Default|GetMain_Player) "0,90.000000, 0" false false)
      (Transformation|SetWorldLocation (Variables|Default|GetCamera) (Math|Vector|MakeVector (+ -4e+02 (+ _xvalue (* 1.0 (Variables|Default|Getspeed)))) 0.0 0.0) false false)
      (CallFunction|SetifIncreasing)
      (Variables|Default|SetIdle_Counter 0))))

(event Input|KeyboardEvents|D
  (params (Key :type Key%20Structure))
  (bind _returnvalue (Transformation|GetActorLocation))
  ;[0.1156 0.3086 1] Movement
  ;;[1 0.1961 0.5725] Right
  (:Pressed
    (if (AI|Components|NavMovement|IsMovingonGround (Variables|Character|GetCharacterMovement))
      (Character|Jump)
      (CallFunction|RoundX)
      (CallFunction|RoundY)
      (Transformation|SetActorRelativeLocation (Math|Vector|MakeVector (.x _returnvalue) (+ (.y _returnvalue) (* -1.0 (Variables|Default|Getspeed))) (.z _returnvalue)) true)
      (Transformation|SetWorldRotation (Variables|Default|GetMain_Player) "0, 0, 0" false false)
      (Variables|Default|SetIdle_Counter 0))))

(event Input|KeyboardEvents|A
  (params (Key :type Key%20Structure))
  ;[0.1156 0.3086 1] Movement
  ;;[1 0.1961 0.5725] Left
  (:Pressed
    (if (AI|Components|NavMovement|IsMovingonGround (Variables|Character|GetCharacterMovement))
      (Character|Jump)
      (bind _xvalue (CallFunction|RoundX))
      (bind _yvalue (CallFunction|RoundY))
      (Transformation|SetActorRelativeLocation (Math|Vector|MakeVector _xvalue (+ _yvalue (* 0.0 (Variables|Default|Getspeed))) (.z (Transformation|GetActorLocation))) true)
      (Transformation|SetWorldRotation (Variables|Default|GetMain_Player) "0,180.000000, 0" false false)
      (Variables|Default|SetIdle_Counter 0))))

(fn ConstructionScript)

(fn RoundY
  (bind _returnvalue (Transformation|GetActorLocation))
  (bind _returnvalue_2 (Math|Float|%(Float) (.y _returnvalue) 2e+02))
  (if (not (>= _returnvalue_2 1e+02))
    (return (- (.y _returnvalue) _returnvalue_2))))

(fn RoundX
  (bind _returnvalue (Transformation|GetActorLocation))
  (bind _returnvalue_2 (Math|Float|%(Float) (.x _returnvalue) 2e+02))
  (if (>= _returnvalue_2 1e+02)
    (return (+ (.x _returnvalue) (- 2e+02 _returnvalue_2)))
    (else
      (return (- (.x _returnvalue) _returnvalue_2)))))

(fn SetifIncreasing
  (bind _outactors (Actor|GetAllActorsOfClass "/Game/Crossy_Content/BluePrints/Global_Variables_BP.Global_Variables_BP_C"))
  (for _array_element _outactors
    (Variables|/Game/Crossy_Content/BluePrints/Global_Variables_BP.Global_Variables_BP_C|SetIs_Increasing _array_element false)))

(fn DeleteLevel
  (bind _outactors (Actor|GetAllActorsOfClass "/Game/Crossy_Content/BluePrints/Global_Variables_BP.Global_Variables_BP_C"))
  (for _array_element _outactors
    (if (>= (Variables|/Game/Crossy_Content/BluePrints/Global_Variables_BP.Global_Variables_BP_C|GetLevel_Score _array_element) 5)
      (if (Variables|/Game/Crossy_Content/BluePrints/Global_Variables_BP.Global_Variables_BP_C|GetIs_Increasing _array_element)
        (for (_array_element_2 _array_index) (Variables|Default|GetStore%20Level%20Names)
          (Development|PrintString (Utilities|String|ToString(Name) _array_element_2))
          (if (== _array_index (Variables|Default|Getcounta))
            (Variables|Default|Setcounta (+ (Variables|Default|Getcounta) 1))
            (Variables|/Game/Crossy_Content/BluePrints/Global_Variables_BP.Global_Variables_BP_C|Setcreate_level _array_element true)))))))

(fn DeathbyEagle
  (bind _outactors (Actor|GetAllActorsOfClass "/Game/Crossy_Content/BluePrints/asset1.asset1_C"))
  (for _array_element _outactors
    (Transformation|SetWorldLocation (Variables|Collision|GetCapsuleComponent) (Transformation|GetWorldLocation (Variables|/Game/Crossy_Content/BluePrints/asset1.asset1_C|GetCartMesh _array_element)) false false)
    (Effects|SpawnEmitteratLocation "/Game/Crossy_Content/Particle_System/Chicken_Death_Blood.Chicken_Death_Blood" (Transformation|GetWorldLocation (Variables|/Game/Crossy_Content/BluePrints/asset1.asset1_C|GetCartMesh _array_element)))))